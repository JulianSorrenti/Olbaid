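; Enemy character that chases the hero, damages it through an overlap box and displays a health bar widget.
; Pawn sensing triggers AI MoveTo, raising a timed attack flag on arrival; behavior tree code is unconnected.
; Any damage subtracts the hero's attack value and briefly freezes movement, flagging death only at exactly zero health.
; Tick polls that flag, then after a delay destroys the actor and decrements the GameMode enemy count.
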(event OnSeePawn(PawnSensing)
  (params (Pawn :type Pawn%20Object%20Reference))
  ;[1 1 1] IA Déplacement ennemi
  (if (not (Variables|Character|GetestMort))
    (AI|AIMoveTo self "0, 0, 0" (Variables|Default|GetHero) 5.0 false
      (:OnSuccess
        (Variables|Character|SetAttaque true)
        (Utilities|FlowControl|Delay 2.6)
        (Variables|Character|SetAttaque false)
        (Development|PrintString (Utilities|String|ToString(Boolean) (Variables|Character|GetAttaque)))))))

(event OnComponentBeginOverlap(BoxDegats)
  (params (OverlappedComponent :type Primitive%20Component%20Object%20Reference) (OtherActor :type Actor%20Object%20Reference) (OtherComp :type Primitive%20Component%20Object%20Reference) (OtherBodyIndex :type Integer) (bFromSweep :type Boolean) (SweepResult :type Hit%20Result%20Structure%20%28by%20ref%29))
  ;[1 1 1] BOX DAMAGE
  (bind _astop_down_character (Utilities|Casting|CastToTopDownCharacter OtherActor))
  (Default|InfligerDegats _astop_down_character (Variables|Character|Getdegats)))

(event Custom|Dead
  ;[1 1 1] Mort Ennemies
  (if (Math|Boolean|Equal(Boolean) (Variables|Character|GetestMort) true)
    (Utilities|FlowControl|Delay 4.0)
    (Actor|DestroyActor)
    (bind _astop_down_game_mode (Utilities|Casting|CastToTopDownGameMode (Game|GetGameMode)))
    (Variables|/Game/TopDownBP/Blueprints/TopDownGameMode.TopDownGameMode_C|SetNombreEnnemis _astop_down_game_mode (- (Variables|/Game/TopDownBP/Blueprints/TopDownGameMode.TopDownGameMode_C|GetNombreEnnemis _astop_down_game_mode) 1))))

(event Game|Damage|EventAnyDamage
  (params (Damage :type Float%20%28single-precision%29) (DamageType :type Damage%20Type%20Object%20Reference) (InstigatedBy :type Controller%20Object%20Reference) (DamageCauser :type Actor%20Object%20Reference))
  ;[1 1 1] Coup infliger par le Hero
  (bind _astop_down_character (Utilities|Casting|CastToTopDownCharacter (Game|GetPlayerCharacter 0)))
  (CallFunction|GestionVieEnnemi (Variables|/Game/TopDownBP/Blueprints/TopDownCharacter.TopDownCharacter_C|GetMouseAttackDamage _astop_down_character))
  (Pawn|Components|CharacterMovement|DisableMovement (Variables|Character|GetCharacterMovement))
  (Components|Movement|StopMovementImmediately (Variables|Character|GetCharacterMovement))
  (Variables|Character|SetTakingDamage true)
  (Utilities|FlowControl|Delay 2.0)
  (Variables|Character|SetTakingDamage false)
  (Pawn|Components|CharacterMovement|SetMovementMode (Variables|Character|GetCharacterMovement) "MOVE_Walking" 0))

(event EventBeginPlay
  ;[1 1 1] Event Begin
  ;;[1 1 1] Instance de la variable hero avec notre caractere principale
  (bind _astop_down_character (Utilities|Casting|CastToTopDownCharacter (Game|GetPlayerCharacter 0)))
  (Variables|Default|SetHero _astop_down_character)
  ;;[1 1 1] Affichage de la vie pour chaque ennemis
  (bind _ashud_vie_ennemi (Utilities|Casting|CastToHUD_VieEnnemi (UserInterface|GetUserWidgetObject (Variables|Default|GetBarre_de_vie))))
  (Variables|/Game/HUD/Ennemi/HUD_VieEnnemi.HUD_VieEnnemi_C|SetEnnemi _ashud_vie_ennemi self))

(event EventTick
  (params (DeltaSeconds :type Float%20%28single-precision%29))
  ;[1 1 1] Action Chaque Tick
  (CallFunction|Dead))

(fn ConstructionScript)

(fn GestionVieEnnemi
  (params (Degats :type Float%20%28single-precision%29))
  (bind _output_get (Variables|Character|SetVieEnnemi (- (Variables|Character|GetVieEnnemi) Degats)))
  (if (== _output_get 0.0)
    (Variables|Character|SetestMort true)))