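; BP_SortDistance is a ranged boss spell actor that damages the player on contact.
; Its Sphere enables query and physics collision shortly after spawn, and the actor destroys itself after a timed lifetime if nothing is hit.
; On overlap with a TopDownCharacter, it calls InfligerDegats on player zero, spawns a fire gib impact emitter at the sphere, then destroys itself.
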(event OnComponentBeginOverlap(Sphere)
  (params (OverlappedComponent :type Primitive%20Component%20Object%20Reference) (OtherActor :type Actor%20Object%20Reference) (OtherComp :type Primitive%20Component%20Object%20Reference) (OtherBodyIndex :type Integer) (bFromSweep :type Boolean) (SweepResult :type Hit%20Result%20Structure%20%28by%20ref%29))
  (if (== (Utilities|GetClass OtherActor) "/Game/TopDownBP/Blueprints/TopDownCharacter.TopDownCharacter_C")
    (bind _astop_down_character (Utilities|Casting|CastToTopDownCharacter (Game|GetPlayerCharacter 0)))
    (Default|InfligerDegats _astop_down_character 5e+01)
    (Effects|SpawnEmitteratLocation "/Game/InfinityBladeEffects/Effects/FX_Mobile/combat/P_Impact_Spider_Gib_Fire.P_Impact_Spider_Gib_Fire" (Transformation|GetWorldLocation (Variables|Default|GetSphere)))
    (Utilities|FlowControl|Delay 0.01)
    (Actor|DestroyActor)))

(event EventBeginPlay
  (Utilities|FlowControl|Delay 0.2)
  (Collision|SetCollisionEnabled (Variables|Default|GetSphere) "QueryAndPhysics")
  (Utilities|FlowControl|Delay 8.0)
  (Actor|DestroyActor))

(event Collision|EventActorBeginOverlap
  (params (OtherActor :type Actor%20Object%20Reference)))

(event EventTick
  (params (DeltaSeconds :type Float%20%28single-precision%29)))

(fn ConstructionScript)