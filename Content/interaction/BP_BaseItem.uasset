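; BP_BaseItem is a world item that the player or another instigator can pick up through an Interaction event.
; On interaction it checks the instigator for inventory space, passes its ItemInfo struct through RamasserMessage, then destroys itself.
; The construction script calls the parent and rebuilds ItemInfo with the actor's own class, keeping the other fields, so the stored data records which class it came from.
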(event EventInteraction
  (params (instigateur :type Top%20Down%20Character%20Object%20Reference))
  (if (Default|HasSpaceinInventory instigateur)
    (Class|BPIInteraction|Ramasser(Message) instigateur (Variables|Default|GetItemInfo))
    (Actor|DestroyActor)))

(fn ConstructionScript
  (|CallParentFunction)
  (Variables|Default|SetItemInfo (Utilities|Struct|MakeItemInfo (.itemtype (Variables|Default|GetItemInfo)) (.itemnom (Variables|Default|GetItemInfo)) (.itemimage (Variables|Default|GetItemInfo)) (Utilities|GetClass self) (.itemindex (Variables|Default|GetItemInfo)) (.itemslot (Variables|Default|GetItemInfo)) (.itemvalue (Variables|Default|GetItemInfo)) (.itemstats (Variables|Default|GetItemInfo)))))