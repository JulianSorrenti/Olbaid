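; BP_Item is an interaction item Blueprint that fills its ItemI struct with randomized numeric values.
; The construction script runs the parent's version, then sets ItemI with fixed enum choices, mostly empty or zero fields, and a nested set of random integers, some converted to floats.
; Values reroll whenever construction runs, and the event graph holds only disabled placeholder events.
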(event EventBeginPlay)

(event Collision|EventActorBeginOverlap
  (params (OtherActor :type Actor%20Object%20Reference)))

(event EventTick
  (params (DeltaSeconds :type Float%20%28single-precision%29)))

(fn ConstructionScript
  (|CallParentFunction)
  (Variables|Default|SetitemI (Utilities|Struct|MakeItemInfo "NewEnumerator1" "" 0 0 0 "NewEnumerator0" 0 (Utilities|Struct|MakeItemStat (Math|Conversions|ToFloat(Integer) (Math|Random|RandomInteger 150)) (Math|Conversions|ToFloat(Integer) (Math|Random|RandomInteger 50)) (Math|Conversions|ToFloat(Integer) (Math|Random|RandomInteger 5)) (Math|Random|RandomInteger 50) (Math|Random|RandomInteger 75) (Math|Random|RandomInteger 30) 0.0) false)))